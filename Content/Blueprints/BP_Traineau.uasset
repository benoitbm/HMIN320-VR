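; BP_Traineau is a VR sleigh that carries the player and tracks their score.
; Each Tick it moves forward at constant speed without sweep and snaps the first BP_VRPawn found at BeginPlay onto its seat point.
; It exposes left/right yaw turning, a weapon origin position and a point-adding event.
; BeginPlay links it to its UW_ScoreTraineau widget and resets the score.
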(event Custom|AjoutPts
  (Math|Integer|IncrementInt (Variables|Default|GetScore)))

(event EventBeginPlay
  ;[0.4247 0.5404 1] Initialisation score
  (bind _asuw_score_traineau (Utilities|Casting|CastToUW_ScoreTraineau (UserInterface|GetUserWidgetObject (Variables|Default|GetWidget))))
  (Variables|/Game/Blueprints/UW_ScoreTraineau.UW_ScoreTraineau_C|SetScoreRef _asuw_score_traineau self)
  (Variables|Default|SetScore 0)
  ;[1 1 1] Référencement du joueur
  (bind _outactors (Actor|GetAllActorsOfClass "/Game/Core/BP_VRPawn.BP_VRPawn_C"))
  (if (Utilities|Array|IsValidIndex _outactors)
    (Variables|Default|SetJoueur (Utilities|Array|Get(acopy) _outactors))))

(event EventTick
  (params (DeltaSeconds :type Float%20%28single-precision%29))
  ;[1 0.4375 0.4375] Avancement constant
  (Transformation|SetWorldLocation (Variables|Default|GetDefaultSceneRoot) (+ (* (* (Math|Vector|GetForwardVector (Transformation|GetActorRotation)) (Variables|Default|GetVitesse)) DeltaSeconds) (Transformation|GetWorldLocation (Variables|Default|GetDefaultSceneRoot))) false false)
  (Utilities|IsValid (Variables|Default|GetJoueur)
    (:Is%20Valid
      ;[1 0.3882 0.826] Replacement du joueur (VR)
      (Transformation|SetWorldLocation (Variables|/Game/Core/BP_VRPawn.BP_VRPawn_C|GetDefaultSceneRoot (Variables|Default|GetJoueur)) (Transformation|GetWorldLocation (Variables|Default|GetPlayperPos)) false false))))

(fn ConstructionScript)

(fn TournerGauche
  (Transformation|AddWorldRotation (Variables|Default|GetDefaultSceneRoot) (* (* "0,-1.000000, 0" (Variables|Default|GetVitesseRotation)) (Utilities|Time|GetWorldDeltaSeconds)) false false))

(fn TournerDroite
  (Transformation|AddWorldRotation (Variables|Default|GetDefaultSceneRoot) (* (* "0,1.000000, 0" (Variables|Default|GetVitesseRotation)) (Utilities|Time|GetWorldDeltaSeconds)) false false))

(fn PosOrigineArme
  (return (Transformation|GetWorldLocation (Variables|Default|GetWeaponPos))))