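; BP_MC is a VR motion controller hand that picks up and drops items, mirroring its hand mesh for the left hand.
; Pickup searches GrabSphere overlaps for PickupActorInterface actors within NearestOverlap distance, keeping the last match since that threshold never updates.
; It sends the found item a pickup message with HandMesh.
; Drop messages the item only if still attached to this hand, otherwise clearing the reference.
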(event Custom|PickupItem
  (bind _nearestactor (CallFunction|FindNearestObjecttoPickup))
  (Utilities|IsValid _nearestactor
    (:Is%20Valid
      (Variables|Default|SetHasGrabbedItem true)
      (bind _output_get (Variables|Default|SetGrabbingItemRef _nearestactor))
      (Class|PickupActorInterface|Pickup(Message) _output_get (Variables|Default|GetHandMesh)))))

(event Custom|DropItem
  (Variables|Default|SetHasGrabbedItem false)
  (Utilities|IsValid (Variables|Default|GetGrabbingItemRef)
    (:Is%20Valid
      (if (== (Transformation|GetAttachParent (Variables|/Script/Engine.Actor|GetRootComponent (Variables|Default|GetGrabbingItemRef))) (Variables|Default|GetHandMesh))
        (Class|PickupActorInterface|Drop(Message) (Variables|Default|GetGrabbingItemRef))
        (else
          (Variables|Default|SetGrabbingItemRef 0))))))

(event EventBeginPlay
  (switch Utilities|FlowControl|Switch|SwitchonEControllerHand (Variables|Default|GetHand)
    (:Left
      (Transformation|SetWorldScale3D (Variables|Default|GetHandMesh) "1.000000,1.000000,-1.000000"))))

(fn ConstructionScript
  (Variables|/Script/HeadMountedDisplay.MotionControllerComponent|SetHand (Variables|Default|GetMotionController) (Variables|Default|GetHand)))

(fn FindNearestObjecttoPickup
  (for _array_element (Collision|GetOverlappingActors (Variables|Default|GetGrabSphere) "/Script/Engine.Actor" :!class /Script/Engine.PrimitiveComponent)
    (if (Utilities|DoesObjectImplementInterface _array_element "/Game/VirtualRealityBP/Blueprints/PickupActorInterface.PickupActorInterface_C")
      (if (< (Math|Vector|VectorLength (- (Transformation|GetActorLocation _array_element) (Transformation|GetWorldLocation (Variables|Default|GetGrabSphere)))) (LocalVariables|GetNearestOverlap))
        (LocalVariables|SetNearestOverlappingActor _array_element))))
  (return (LocalVariables|GetNearestOverlappingActor)))