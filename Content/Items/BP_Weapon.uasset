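; BP_Weapon is a weapon item that can be picked up and dropped, with its mesh SMWeapon switching physics to match.
; Pickup stops physics simulation and snaps the mesh to the WeaponSocket of the given component, keeping relative scale.
; If that component's owner is a BP_MC set to the left hand, the mesh yaw is flipped.
; Drop re-enables physics and detaches the actor, keeping its world transform.
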(event EventDrop
  (Physics|SetSimulatePhysics (Variables|Default|GetSM_Weapon) true)
  (Transformation|DetachFromActor "KeepWorld" "KeepWorld" "KeepWorld"))

(event EventPickup
  (params (AttachTo :type Scene%20Component%20Object%20Reference))
  (bind _sm_weapon (Variables|Default|GetSM_Weapon))
  (Physics|SetSimulatePhysics _sm_weapon false)
  (Transformation|AttachComponentToComponent _sm_weapon AttachTo "WeaponSocket" "SnapToTarget" "SnapToTarget" "KeepRelative" false)
  (bind _asbp_mc (Utilities|Casting|CastToBP_MC (Components|GetOwner AttachTo)))
  (if (Utilities|Enum|Equal(Enum) (Variables|/Game/Core/BP_MC.BP_MC_C|GetHand _asbp_mc) "Left")
    (Transformation|SetRelativeRotation (Variables|Default|GetSM_Weapon) "180.000000, 0, 0" false false)))

(fn ConstructionScript)